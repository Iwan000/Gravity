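; Blackhole-reactive platform actor that detects when a gravity well bullet's interact sphere enters or leaves its Box volume.
; Overlap start prints a debug "Black" message and calls Trigger, which is empty here; overlap end calls Strigger after a short delay.
; BeginPlay caches the PolarityRun actor, a whitehole bullet actor and the Cube's world location, none of which are used in this graph.
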(event OnComponentEndOverlap(Box)
  (params (OverlappedComponent :type Primitive%20Component%20Object%20Reference) (OtherActor :type Actor%20Object%20Reference) (OtherComp :type Primitive%20Component%20Object%20Reference) (OtherBodyIndex :type Integer))
  (bind _asbp_gravity_well_actor_bullet (Utilities|Casting|CastToBP_GravityWellActor_Bullet OtherActor))
  (if (== OtherComp (Variables|/Game/Blueprints/BP_GravityWellActor_Bullet.BP_GravityWellActor_Bullet_C|GetInteractSphere _asbp_gravity_well_actor_bullet))
    (Utilities|FlowControl|Delay 2.0)
    (CallFunction|Strigger)))

(event OnComponentBeginOverlap(Box)
  (params (OverlappedComponent :type Primitive%20Component%20Object%20Reference) (OtherActor :type Actor%20Object%20Reference) (OtherComp :type Primitive%20Component%20Object%20Reference) (OtherBodyIndex :type Integer) (bFromSweep :type Boolean) (SweepResult :type Hit%20Result%20Structure%20%28by%20ref%29))
  (bind _asbp_gravity_well_actor_bullet (Utilities|Casting|CastToBP_GravityWellActor_Bullet OtherActor))
  (if (== OtherComp (Variables|/Game/Blueprints/BP_GravityWellActor_Bullet.BP_GravityWellActor_Bullet_C|GetInteractSphere _asbp_gravity_well_actor_bullet))
    (Development|PrintString "Black")
    (CallFunction|Trigger)))

(event Custom|Trigger)

(event EventBeginPlay
  (bind _returnvalue (Actor|GetActorOfClass "/Game/BP_PolarityRun.BP_PolarityRun_C"))
  (Variables|Default|SetBP_PolarityRun _returnvalue)
  (bind _returnvalue_2 (Actor|GetActorOfClass "/Game/Blueprints/BP_Whitehole_Actor_Bullet.BP_Whitehole_Actor_Bullet_C"))
  (Variables|Default|SetBP_Whitehole _returnvalue_2)
  (Variables|Default|SetLocation (Transformation|GetWorldLocation (Variables|Default|GetCube))))

(event Collision|EventActorBeginOverlap
  (params (OtherActor :type Actor%20Object%20Reference)))

(event EventTick
  (params (DeltaSeconds :type Float%20%28single-precision%29)))

(fn ConstructionScript)